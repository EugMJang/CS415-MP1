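; BP_TunnelSpawner builds the chain of BP_Tunnel segments that forms the level, starting at the player pawn's location.
; On BeginPlay it destroys any existing tunnels, then spawns a short starting run, attaching each new segment at the previous one's SpawnPoint.
; Each tunnel gets a reference back to the spawner and a randomized wall; all but the first also get a randomized pack.
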(event EventBeginPlay
  (CallFunction|SpawnInitialTunnels))

(event Collision|EventActorBeginOverlap
  (params (OtherActor :type Actor%20Object%20Reference)))

(event EventTick
  (params (DeltaSeconds :type Float%20%28single-precision%29)))

(fn ConstructionScript)

(fn SpawnTunnel
  (params (SpawnLocation :type Vector) (FirstTunnels :type Boolean))
  (bind _returnvalue (Game|SpawnActorfromClass "/Game/InfiniteMatrix/Blueprints/BP_Tunnel.BP_Tunnel_C" (Math|Transform|MakeTransform SpawnLocation "0, 0, 0" "1,1,1") "Undefined" 0 0))
  (bind _output_get (Variables|Default|SetNewestTunnel _returnvalue))
  (Variables|/Game/InfiniteMatrix/Blueprints/BP_Tunnel.BP_Tunnel_C|SetTunnelSpawner _output_get self)
  (Default|RandomizeWall _output_get)
  (if (not FirstTunnels)
    (Default|RandomizePack _output_get)))

(fn SpawnTunnelatSpawnPoint
  (CallFunction|SpawnTunnel (Transformation|GetWorldLocation (Variables|/Game/InfiniteMatrix/Blueprints/BP_Tunnel.BP_Tunnel_C|GetSpawnPoint (Variables|Default|GetNewestTunnel))) false))

(fn SpawnInitialTunnels
  (Utilities|FlowControl|Sequence
    (:then_0
      (bind _outactors (Actor|GetAllActorsOfClass "/Game/InfiniteMatrix/Blueprints/BP_Tunnel.BP_Tunnel_C"))
      (for _array_element _outactors
        (Actor|DestroyActor _array_element)))
    (:then_1
      (for _index (range 0 2)
        (Utilities|IsValid (Variables|Default|GetNewestTunnel)
          (:Is%20Valid
            (CallFunction|SpawnTunnelatSpawnPoint))
          (:Is%20Not%20Valid
            (CallFunction|SpawnTunnel (Transformation|GetActorLocation (Game|Player|GetPlayerPawn 0)) true)))))))